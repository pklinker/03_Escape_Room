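; Openable door Blueprint that swings the actor open and closed in response to OpenDoor's OnOpen and OnClose events.
; The DoorSwing timeline drives an OpenYaw offset, combined with the rotation cached on BeginPlay, to rotate the whole actor.
; Opening plays the timeline with a Sound Timing event track that triggers a door lock sound at the actor's location, and closing reverses it.
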(event `self.OpenDoor.OnOpen`
  (bind (_direction _open_yaw) (`Timeline|Door Swing` :!label _label)
    (:`Update`
      (`self.K2_SetActorRotation` (`KismetMathLibrary.ComposeRotators` (`KismetMathLibrary.MakeRotator` 0.0 0.0 _open_yaw) (`self.InitialRotation`))))
    (:`Sound Timing`
      (`GameplayStatics.PlaySoundAtLocation` "/Game/Audio/door-lock.door-lock" (`self.K2_GetActorLocation`) (struct) 1.0 1.0 0.0 null null null))))

(event `self.OpenDoor.OnClose`
  (goto _label :!via `Reverse`))

(event `self.ReceiveBeginPlay`
  (set `self.InitialRotation` (`self.K2_GetActorRotation`)))

(fn `UserConstructionScript`)